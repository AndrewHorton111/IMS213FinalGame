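; BP_Wind is a wind volume that floats the player upward while inside it.
; Overlapping its RangeBox with a BP_ThirdPersonCharacter starts a looping 60 Hz timer that applies small, additive upward LaunchCharacter impulses.
; A flag and delay throttle the 2D wind sound.
; Any actor ending overlap clears the launch flag, but the timer is never cleared.
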(event OnComponentBeginOverlap(RangeBox)
  (params (OverlappedComponent :type Primitive%20Component%20Object%20Reference) (OtherActor :type Actor%20Object%20Reference) (OtherComp :type Primitive%20Component%20Object%20Reference) (OtherBodyIndex :type Integer) (bFromSweep :type Boolean) (SweepResult :type Hit%20Result%20Structure%20%28by%20ref%29))
  ;[1 1 1] Makes the player float upwards while in wind
  (bind _asbp_third_person_character (Utilities|Casting|CastToBP_ThirdPersonCharacter OtherActor))
  (Variables|Default|SetPlayer _asbp_third_person_character)
  (Variables|Default|SetShouldLaunch true)
  (Utilities|Time|SetTimerbyEvent (delegate Custom|Wind) 0.016667 (Variables|Default|GetShouldLaunch)))

(event Custom|Wind
  ;[1 1 1] Makes the player float upwards while in wind
  (if (Variables|Default|GetShouldLaunch)
    (Character|LaunchCharacter (Variables|Default|GetPlayer) "0.000000,0.000000,28.500000" false false)
    (if (Variables|Default|GetPlaySound)
      (Audio|PlaySound2D "/Game/Sounds/Wind.Wind" 1.0 1.0 0.0 0 0)
      (Variables|Default|SetPlaySound false)
      (Utilities|FlowControl|Delay 0.7)
      (Variables|Default|SetPlaySound true))))

(event Collision|EventActorBeginOverlap
  (params (OtherActor :type Actor%20Object%20Reference)))

(event Collision|EventActorEndOverlap
  (params (OtherActor :type Actor%20Object%20Reference))
  ;[1 1 1] Makes the player float upwards while in wind
  (Variables|Default|SetShouldLaunch false))

(fn ConstructionScript)