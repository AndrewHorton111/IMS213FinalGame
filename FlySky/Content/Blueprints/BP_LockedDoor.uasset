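; BP_LockedDoor is a double door that slides open when its UnlockDoor event is called.
; BeginPlay caches each panel's starting world X, plus the left panel's Y and Z for both.
; After a short delay, UnlockDoor plays the OpenTheDoor timeline, whose GarageDoorPosition track moves the panels apart in opposite directions along world X.
; The file contains no lock check or closing logic.
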(event Custom|UnlockDoor
  ;[1 1 1] Opens the door
  (Utilities|FlowControl|Delay 0.25)
  (bind _garagedoorposition (Timeline|OpenTheDoor PlayFromStart)
    (:Update
      (Transformation|SetWorldLocation (Variables|Default|GetDoorLeft) (Math|Vector|MakeVector (- (Variables|Default|GetStartX_Left) _garagedoorposition) (Variables|Default|GetStartY) (Variables|Default|GetStartZ)) false false)
      (Transformation|SetWorldLocation (Variables|Default|GetDoorRight) (Math|Vector|MakeVector (+ _garagedoorposition (Variables|Default|GetStartX_Right)) (Variables|Default|GetStartY) (Variables|Default|GetStartZ)) false false))))

(event EventBeginPlay
  (bind _doorleft (Variables|Default|GetDoorLeft))
  (bind _returnvalue (Transformation|GetWorldLocation _doorleft))
  ;[1 1 1] Gets position of the door
  (Variables|Default|SetStartX_Left (.x _returnvalue))
  (Variables|Default|SetStartY (.y _returnvalue))
  (Variables|Default|SetStartZ (.z _returnvalue))
  (Variables|Default|SetStartX_Right (.x (Transformation|GetWorldLocation (Variables|Default|GetDoorRight)))))

(fn ConstructionScript)